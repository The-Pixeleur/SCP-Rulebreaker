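; Player blink component that drains a blink meter and tracks whether the player can see.
; A looping timer lowers BeforeBlink, with a one-time delay when full, and calls Blink with false at zero.
; Blink only acts on true, spawning one UMG_Blinking widget linked back to the component.
; EndBlink refills the meter and re-arms blinking, while Tick sets CanSee opposite to Blinking.
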(event `self.ReceiveBeginPlay`
  (`KismetSystemLibrary.K2_SetTimerDelegate` (delegate `BeforeBlinkLoop`) 0.1 true))

(event `BeforeBlinkLoop`
  (if (== (`self.BeforeBlinkMax`) (`self.BeforeBlink`))
    (`/Engine/EditorBlueprintResources/StandardMacros.DoOnce` false :!label _label
      (:`Completed`
        (`KismetSystemLibrary.Delay` (`self.BeforeBlinkDelay`))))
    (else
      (`|ExecutionSequence`
        (:`then_0`
          (goto _label :!via `Reset`))
        (:`then_1`
          _))))
  (bind _output_get (set `self.BeforeBlink` (- (`self.BeforeBlink`) (`self.BeforeBlinkDrain`))))
  (if (<= _output_get 0.0)
    (`self.Blink` false)))

(event `Blink`
  (params (`ShouldBlink?` :type Boolean))
  (if `ShouldBlink?`
    (`/Engine/EditorBlueprintResources/StandardMacros.DoOnce` false :!label _label_2
      (:`Completed`
        (set `self.Blinking?` true)
        (bind _returnvalue (`|CreateWidget` "/Game/UI/UMG_Blinking.UMG_Blinking_C"))
        (set `/Game/UI/UMG_Blinking.BlinkComponent` self _returnvalue)
        (`UserWidget.AddToPlayerScreen` _returnvalue 0)))))

(event `EndBlink`
  (set `self.Blinking?` false)
  (set `self.BeforeBlink` (`self.BeforeBlinkMax`))
  (goto _label_2 :!via `Reset`))

(event `self.ReceiveTick`
  (params (DeltaSeconds :type "Float (single-precision)"))
  (set `self.CanSee?` (not (`self.Blinking?`))))