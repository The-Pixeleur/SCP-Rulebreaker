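; Class-D AI character that spawns a knife in its right hand and stabs the player or other AI.
; Attacking plays a stab animation while a delayed line trace from the knife passes its hit actor to DamageTarget, which casts to supported victim types.
; Perception updates and Settarget write the target and its location to the Blackboard.
; Damage and Kill feed IsDead, which destroys the knife and character when health runs out.
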(event `self.ReceiveBeginPlay`
  (bind _returnvalue (`|SpawnActorFromClass` "/Game/Meshes/Props/Knife/BP_Knife.BP_Knife_C" (`KismetMathLibrary.MakeTransform` (0.0 0.0 0.0)) "Undefined" "OverrideRootScale" null null))
  (bind _output_get (set `self.knife_ref` _returnvalue))
  (`SceneComponent.K2_AttachToComponent` (`/Game/Meshes/Props/Knife/BP_Knife.StaticMesh` _output_get) (`self.Mesh`) "righthand" "SnapToTarget" "SnapToTarget" "SnapToTarget" true))

(event `Attacking`
  (bind _knife_ref (`self.knife_ref`))
  (`|ExecutionSequence`
    (:`then_0`
      (`KismetSystemLibrary.Delay` 0.5)
      (bind _outhit (`KismetSystemLibrary.LineTraceSingle` (`SceneComponent.K2_GetComponentLocation` (`/Game/Meshes/Props/Knife/BP_Knife.StaticMesh` _knife_ref)) (* (`self.GetActorForwardVector` _knife_ref) 100.0) "TraceTypeQuery1" false (`|MakeArray` self :!type "Actor Object Reference") "None" true (struct :`R` 0.453125 :`A` 1.0)))
      (`self.DamageTarget` (`.HitActor` (`GameplayStatics.BreakHitResult` _outhit))))
    (:`then_1`
      (`SkeletalMeshComponent.PlayAnimation` (`self.Mesh`) "/Game/AI/FoundationStaff/Placeholder/Stabbing_PlaceHolder.Stabbing_PlaceHolder" false)
      (`KismetSystemLibrary.Delay` 2.133)
      (`SkeletalMeshComponent.SetAnimationMode` (`self.Mesh`) "AnimationBlueprint"))))

(event `Damage`
  (params (calibe :type "/Game/Blueprint/Weapon/enum_Caliber Enum" :default "NewEnumerator0") (VieToRemove :type "Float (double-precision)"))
  (bind _vie (`self.Vie`))
  (if (not (<= _vie 0.0))
    (set `self.Vie` (- _vie VieToRemove))
    (`self.IsDead?`)))

(event `IsDead?`
  (bind _mesh (`self.Mesh`))
  (if (<= (`self.Vie`) 0.0)
    (set `self.dead?` true)
    (set `CharacterMovementComponent.MaxWalkSpeed` 0.0 (`self.CharacterMovement`))
    (`PrimitiveComponent.SetSimulatePhysics` _mesh true)
    (`PrimitiveComponent.SetCollisionEnabled` (`self.CapsuleComponent`) "NoCollision")
    (`SkeletalMeshComponent.SetPlayRate` _mesh 0.0)
    (`SkeletalMeshComponent.Stop` _mesh)
    (`self.K2_DestroyActor` (`self.knife_ref`))
    (`self.K2_DestroyActor`)))

(event `Kill`
  (set `self.Vie` 0.0)
  (`self.IsDead?`))

(event `self.AIPerception.OnTargetPerceptionUpdated`
  (params (Actor :type "Actor Object Reference") (Stimulus :type "AIStimulus Structure"))
  (bind _returnvalue (`AIBlueprintHelperLibrary.GetBlackboard` null))
  (`BlackboardComponent.SetValueAsObject` _returnvalue (`self.Key Name`) Actor)
  (`BlackboardComponent.SetValueAsVector` _returnvalue (`self.Range`) (`self.K2_GetActorLocation` Actor)))

(event `Settarget`
  (params (ObjectValue :type "Actor Object Reference"))
  (`BlackboardComponent.SetValueAsObject` (`AIBlueprintHelperLibrary.GetBlackboard` null) (`self.Key Name`) ObjectValue)
  (`BlackboardComponent.SetValueAsVector` (`AIBlueprintHelperLibrary.GetBlackboard` null) (`self.Range`) (`self.K2_GetActorLocation` ObjectValue)))

(fn `DamageTarget`
  (params (Object :type "Actor Object Reference"))
  (bind _asfirst_person_character (cast `/Game/PlayerBP/Blueprints/FirstPersonCharacter` Object)
    (:`then`
      (`/Game/PlayerBP/Blueprints/FirstPersonCharacter.Damage` _asfirst_person_character "NewEnumerator0" true false 10.0))
    (:`CastFailed`
      (bind _asbp_fim_e_11 (cast `/Game/AI/FoundationStaff/FIM/E-11/BP_FIM-e11` Object)
        (:`then`
          (`/Game/AI/FoundationStaff/FIM/E-11/BP_FIM-e11.Damage` _asbp_fim_e_11 "NewEnumerator0" true))
        (:`CastFailed`
          (bind _asbp_friendly_gunner_ai (cast `/Game/AI/FoundationStaff/BP_FriendlyGunnerAI` Object))
          (`/Game/AI/FoundationStaff/BP_FriendlyGunnerAI.Damage` _asbp_friendly_gunner_ai "NewEnumerator0" true))))))

(fn `UserConstructionScript`)