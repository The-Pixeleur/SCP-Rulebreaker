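; Friendly Foundation staff gunner pawn that spawns with a random weapon from its list and fires on Class-D characters.
; Shoot waits for reload or fire rate, then fires only if a muzzle line trace hits the cached Class-D, caching the first one hit.
; Focus aims the AI controller at a given actor.
; Damage distinguishes knife from other hits; death swaps the weapon for a pickup retaining class and ammo, then destroys the actor.
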(event `Damage`
  (params (calibe :type "/Game/Blueprint/Weapon/enum_Caliber Enum" :default "NewEnumerator0") (`knife?` :type Boolean))
  (bind _vie (`self.Vie`))
  (bind _vie_2 (`self.Vie`))
  (if `knife?`
    (if (not (<= _vie_2 0.0))
      (set `self.Vie` (- _vie_2 75.0))
      (`self.IsDead?` :!label _label))
    (elif (not (<= _vie 0.0))
      (set `self.Vie` (- _vie 34.0))
      (goto _label))))

(event `IsDead?`
  (bind _weaponref (`self.WeaponRef`))
  (bind _mesh (`self.Mesh`))
  (bind (_returnvalue_location _returnvalue_rotation) (`KismetMathLibrary.BreakTransform` (`self.GetTransform` _weaponref)))
  (if (<= (`self.Vie`) 0.0)
    (set `self.dead?` true)
    (set `CharacterMovementComponent.MaxWalkSpeed` 0.0 (`self.CharacterMovement`))
    (`PrimitiveComponent.SetSimulatePhysics` _mesh true)
    (`PrimitiveComponent.SetCollisionEnabled` (`self.CapsuleComponent`) "NoCollision")
    (`SkeletalMeshComponent.SetPlayRate` _mesh 0.0)
    (`SkeletalMeshComponent.Stop` _mesh)
    (bind _returnvalue (`|SpawnActorFromClass` "/Game/Blueprint/Object/Weapon/BP_WeaponToGrab_Master.BP_WeaponToGrab_Master_C" (`KismetMathLibrary.MakeTransform` _returnvalue_location _returnvalue_rotation) "Undefined" "OverrideRootScale" null null))
    (set `/Game/Blueprint/Object/Weapon/BP_WeaponToGrab_Master.NewWeaponStruct` (make `/Game/Blueprint/Object/Weapon/S_WeaponGrab` (`/Game/Blueprint/Weapon/BP_Weapon_Master.AmmoCurrent` _weaponref) (`GameplayStatics.GetObjectClass` _weaponref)) _returnvalue)
    (`/Engine/EditorBlueprintResources/StandardMacros.IsValid` (`/Game/Blueprint/Object/Weapon/BP_WeaponToGrab_Master.Weapon` _returnvalue)
      (:`Is Valid`
        _)
      (:`Is Not Valid`
        (`/Game/Blueprint/Object/Weapon/BP_WeaponToGrab_Master.AddWeapon` _returnvalue)))
    (`self.K2_DestroyActor` _weaponref)
    (`self.K2_DestroyActor`)))

(event `Kill`
  (set `self.Vie` 0.0)
  (`self.IsDead?`))

(event `self.ReceiveBeginPlay`
  (`self.NewWeapon` (`KismetArrayLibrary.Array_Random` (`self.WeaponList`))))

(event `Shoot`
  (params (`HowManyAmmo?` :type Integer))
  (bind _weaponref (`self.WeaponRef`))
  (bind _dead_ (`self.dead?`))
  (if (`self.dead?`)
    _
    (elif (`self.dead?`)
      _
      (elif (`/Game/Blueprint/Weapon/BP_Weapon_Master.Reloading?` _weaponref)
        (`KismetSystemLibrary.Delay` (`/Game/Blueprint/Weapon/BP_Weapon_Master.ReloadTime` _weaponref))
        (if (not _dead_)
          (bind _canshoot_ (`self.CanShoot?` :!label _label_2))
          (if _canshoot_
            (`/Game/Blueprint/Weapon/BP_Weapon_Master.Shooting` _weaponref false self)))
        (else
          (`KismetSystemLibrary.Delay` (/ 1.0 (/ (`/Game/Blueprint/Weapon/BP_Weapon_Master.RoundPerMinutes` _weaponref) 60.0)))
          (if (not _dead_)
            (goto _label_2)))))))

(event `NewWeapon`
  (params (Struc_Ref :type "/Game/Blueprint/Object/Weapon/S_WeaponGrab Structure"))
  (bind (_ammocurrent _weaponcurrent _topattachment _sideattachment _bottomattachment _tipattachment _topattachment_transform _sideattachment_transform _bottomattachment_transform _tipattachment_transform) (break `/Game/Blueprint/Object/Weapon/S_WeaponGrab` Struc_Ref))
  (bind _weaponref (`self.WeaponRef`))
  (`/Engine/EditorBlueprintResources/StandardMacros.IsValid` _weaponref
    (:`Is Valid`
      (`self.K2_DestroyActor` _weaponref))
    (:`Is Not Valid`
      _))
  (`self.SpawnWeapon` _weaponcurrent _ammocurrent _topattachment _sideattachment _bottomattachment _tipattachment _topattachment_transform _sideattachment_transform _bottomattachment_transform _tipattachment_transform)
  (`self.SetActorEnableCollision` _weaponref false))

(event `SpawnWeapon`
  (params (WeaponToSpawn :type "/Game/Blueprint/Weapon/BP_Weapon_Master Class Reference") (Ammo :type Integer) (Top :type "StaticMesh Object Reference") (Side :type "StaticMesh Object Reference") (Bottom :type "StaticMesh Object Reference") (Tip :type "StaticMesh Object Reference") (TopTransform :type "Transform Structure") (SideTransform :type "Transform Structure") (BottomTransform :type "Transform Structure") (TipTransform :type "Transform Structure"))
  (bind _weaponref (`self.WeaponRef`))
  (bind _weaponref_2 (`self.WeaponRef`))
  (bind _weaponref_3 (`self.WeaponRef`))
  (bind _weaponref_4 (`self.WeaponRef`))
  (bind _returnvalue (`|SpawnActorFromClass` WeaponToSpawn (`SceneComponent.GetSocketTransform` (`self.Mesh`) "WeaponRightSocket" "RTS_World") "Undefined" "OverrideRootScale" null null))
  (bind _output_get (set `self.WeaponRef` _returnvalue))
  (`SceneComponent.K2_AttachToComponent` (`Actor.RootComponent` _output_get) (`self.Mesh`) "WeaponRightSocket" "SnapToTarget" "SnapToTarget" "SnapToTarget" true)
  (set `/Game/Blueprint/Weapon/BP_Weapon_Master.AmmoCurrent` Ammo _output_get)
  (`|ExecutionSequence`
    (:`then_0`
      (`/Engine/EditorBlueprintResources/StandardMacros.IsValid` Top
        (:`Is Valid`
          (`/Game/Blueprint/Weapon/BP_Weapon_Master.SetAttachment` _weaponref_4 (`/Game/Blueprint/Weapon/BP_Weapon_Master.TopAttachment` _weaponref_4) Top TopTransform))))
    (:`then_1`
      (`/Engine/EditorBlueprintResources/StandardMacros.IsValid` Side
        (:`Is Valid`
          (`/Game/Blueprint/Weapon/BP_Weapon_Master.SetAttachment` _weaponref_3 (`/Game/Blueprint/Weapon/BP_Weapon_Master.SideAttachment` _weaponref_3) Side SideTransform))))
    (:`then_2`
      (`/Engine/EditorBlueprintResources/StandardMacros.IsValid` Bottom
        (:`Is Valid`
          (`/Game/Blueprint/Weapon/BP_Weapon_Master.SetAttachment` _weaponref_2 (`/Game/Blueprint/Weapon/BP_Weapon_Master.BottomAttachment` _weaponref_2) Bottom BottomTransform))))
    (:`then_3`
      (`/Engine/EditorBlueprintResources/StandardMacros.IsValid` Tip
        (:`Is Valid`
          (`/Game/Blueprint/Weapon/BP_Weapon_Master.SetAttachment` _weaponref (`/Game/Blueprint/Weapon/BP_Weapon_Master.TipAttachment` _weaponref) Tip TipTransform))))))

(event `Focus`
  (params (InFocusActor :type "Actor Object Reference"))
  (bind _returnvalue (`AIBlueprintHelperLibrary.GetAIController` self))
  (`/Engine/EditorBlueprintResources/StandardMacros.IsValid` InFocusActor
    (:`Is Valid`
      (`AIController.K2_SetFocus` _returnvalue InFocusActor)
      (`AIController.K2_SetFocalPoint` _returnvalue (`self.K2_GetActorLocation` InFocusActor)))))

(fn `CanShoot?`
  (returns (`CanShoot?` :type Boolean))
  (bind _weaponref (`self.WeaponRef`))
  (bind _weaponref_2 (`self.WeaponRef`))
  (bind _returnvalue (`SceneComponent.K2_GetComponentLocation` (`/Game/Blueprint/Weapon/BP_Weapon_Master.SphereLineTrace` _weaponref_2)))
  (bind _returnvalue_2 (`SceneComponent.K2_GetComponentLocation` (`/Game/Blueprint/Weapon/BP_Weapon_Master.SphereLineTrace` _weaponref)))
  (`/Engine/EditorBlueprintResources/StandardMacros.IsValid` (`self.dclassref`)
    (:`Is Valid`
      (bind _outhit (`KismetSystemLibrary.LineTraceSingle` _returnvalue (+ _returnvalue (* (`SceneComponent.GetForwardVector` (`/Game/Blueprint/Weapon/BP_Weapon_Master.SphereLineTrace` _weaponref_2)) (`/Game/Blueprint/Weapon/BP_Weapon_Master.WeaponRange` _weaponref_2))) "TraceTypeQuery1" false (`|MakeArray` self :!type "Actor Object Reference") "ForOneFrame"))
      (if (== (`.HitActor` (`GameplayStatics.BreakHitResult` _outhit)) (`self.dclassref`))
        (return true)
        (else
          (return false))))
    (:`Is Not Valid`
      (bind _outhit_2 (`KismetSystemLibrary.LineTraceSingle` _returnvalue_2 (+ _returnvalue_2 (* (`SceneComponent.GetForwardVector` (`/Game/Blueprint/Weapon/BP_Weapon_Master.SphereLineTrace` _weaponref)) (`/Game/Blueprint/Weapon/BP_Weapon_Master.WeaponRange` _weaponref))) "TraceTypeQuery1" false (`|MakeArray` self :!type "Actor Object Reference") "ForOneFrame"))
      (bind _asbp_classe_d (cast `/Game/AI/FoundationStaff/ClasseD/BP_ClasseD` (`.HitActor` (`GameplayStatics.BreakHitResult` _outhit_2)))
        (:`then`
          (set `self.dclassref` _asbp_classe_d)
          (return true))
        (:`CastFailed`
          (return false))))))

(fn `GetWeaponSocketTransform`
  (params (SocketName :type Name))
  (returns (SocketTransform :type "Transform Structure"))
  (bind _weaponref (`self.WeaponRef`))
  (`/Engine/EditorBlueprintResources/StandardMacros.IsValid` _weaponref
    (:`Is Valid`
      (if (`/Game/Blueprint/Weapon/BP_Weapon_Master.AsBottomAttachment?` _weaponref)
        (return (`SceneComponent.GetSocketTransform` (`/Game/Blueprint/Weapon/BP_Weapon_Master.BottomAttachment` _weaponref) SocketName "RTS_World"))
        (else
          (return (`SceneComponent.GetSocketTransform` (`/Game/Blueprint/Weapon/BP_Weapon_Master.WeaponBody` _weaponref) SocketName "RTS_World")))))))

(fn `SetAdsPos`
  (returns (ADStransform :type "Transform Structure"))
  (return))

(fn `SetRecoilHands`
  (returns (RecoilNewPos :type "Transform Structure"))
  (bind _weaponref (`self.WeaponRef`))
  (`/Engine/EditorBlueprintResources/StandardMacros.IsValid` _weaponref
    (:`Is Valid`
      (return (`/Game/Blueprint/Weapon/BP_Weapon_Master.RecoilTransformDNC` _weaponref)))))

(fn `UserConstructionScript`)