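; BP_096 is the SCP-096 actor, which reacts to the player looking at it while SCRAMBLES is activated.
; Each tick, a view-direction dot product and a visibility trace test whether the camera sees its Sphere, raising audio exponentially as aim centers and otherwise fading it out.
; ScrambleCheck, run at BeginPlay, shows or hides four material billboards based on the SCRAMBLES state.
; Enrage is only a debug-print stub.
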(event `self.ReceiveBeginPlay`
  (bind _asfirst_person_character (cast `/Game/PlayerBP/Blueprints/FirstPersonCharacter` (`GameplayStatics.GetPlayerPawn` 0)))
  (set `self.As First Person Character` _asfirst_person_character)
  (`self.ScrambleCheck`))

(event `self.ReceiveTick`
  (params (DeltaSeconds :type "Float (single-precision)"))
  (bind _audio (`self.Audio`))
  (bind _firstpersoncamera (`/Game/PlayerBP/Blueprints/FirstPersonCharacter.FirstPersonCamera` (`self.As First Person Character`)))
  (bind _returnvalue (* (`KismetMathLibrary.Dot_VectorVector` (`KismetMathLibrary.GetForwardVector` (`KismetMathLibrary.FindLookAtRotation` (`SceneComponent.K2_GetComponentLocation` (`self.Sphere`)) (`SceneComponent.K2_GetComponentLocation` _firstpersoncamera))) (`SceneComponent.GetForwardVector` _firstpersoncamera)) -10.0))
  (if (>= _returnvalue 8.0)
    (bind _outhit (`KismetSystemLibrary.LineTraceSingle` :`Start` (`SceneComponent.K2_GetComponentLocation` (`/Game/PlayerBP/Blueprints/FirstPersonCharacter.FirstPersonCamera` (`self.As First Person Character`))) :`End` (`SceneComponent.K2_GetComponentLocation` (`self.Sphere`)) :`TraceChannel` "TraceTypeQuery1" :`bTraceComplex` true :`DrawDebugType` "ForDuration" :`bIgnoreSelf` false))
    (if (== (`self.Sphere`) (`.HitComponent` (`GameplayStatics.BreakHitResult` _outhit)))
      (if (`/Game/PlayerBP/Blueprints/FirstPersonCharacter.SCRAMBLESactivated?` (`self.As First Person Character`))
        (`AudioComponent.AdjustVolume` _audio 0.1 (* (`KismetMathLibrary.MultiplyMultiply_FloatFloat` 10.0 (/ (- _returnvalue 10.0) 3.0)) 1.5) "Linear")
        (else
          (`AudioComponent.AdjustVolume` _audio 0.2 0.001 "Linear" :!label _label)))
      (else
        (goto _label)))
    (else
      (`AudioComponent.AdjustVolume` (`self.Audio`) 0.2 0.001 "Linear"))))

(fn `Enrage`
  (`KismetSystemLibrary.PrintString` "Hello"))

(fn `ScrambleCheck`
  (bind _materialbillboard2 (`self.MaterialBillboard2`))
  (bind _asfirst_person_character (cast `/Game/PlayerBP/Blueprints/FirstPersonCharacter` (`GameplayStatics.GetPlayerPawn` 0)))
  (if (`/Game/PlayerBP/Blueprints/FirstPersonCharacter.SCRAMBLESactivated?` _asfirst_person_character)
    (`SceneComponent.SetVisibility` _materialbillboard2 true false)
    (`SceneComponent.SetVisibility` (`self.MaterialBillboard`) true false)
    (`SceneComponent.SetVisibility` (`self.MaterialBillboard1`) true false)
    (`SceneComponent.SetVisibility` (`self.MaterialBillboard3`) true false)
    (else
      (`SceneComponent.SetVisibility` _materialbillboard2 false false)
      (`SceneComponent.SetVisibility` (`self.MaterialBillboard`) false false)
      (`SceneComponent.SetVisibility` (`self.MaterialBillboard1`) false false)
      (`SceneComponent.SetVisibility` (`self.MaterialBillboard3`) false false))))

(fn `UserConstructionScript`)