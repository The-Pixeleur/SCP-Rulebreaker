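; BP_SCP-173 is the SCP-173 AI pawn, which plays a movement sound and threatens the player on contact.
; Tick plays the audio component while velocity is nonzero and stops it when stationary.
; A sphere overlap with FirstPersonCharacter reads the Canmove blackboard key and, if true, prints a death message as a placeholder kill.
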(event `self.ReceiveTick`
  (params (DeltaSeconds :type "Float (single-precision)"))
  (bind _audio (`self.Audio`))
  (if (== (`self.GetVelocity`) (0.0 0.0 0.0))
    (`AudioComponent.Stop` _audio)
    (elif (not (`AudioComponent.IsPlaying` _audio))
      (`AudioComponent.Play` _audio 0.0))))

(event `self.Sphere.OnComponentBeginOverlap`
  (params (OverlappedComponent :type "PrimitiveComponent Object Reference") (OtherActor :type "Actor Object Reference") (OtherComp :type "PrimitiveComponent Object Reference") (OtherBodyIndex :type Integer) (bFromSweep :type Boolean) (SweepResult :type "HitResult Structure (by ref)"))
  (set `self.CanMove?` (`BlackboardComponent.GetValueAsBool` (`AIBlueprintHelperLibrary.GetBlackboard` self) (`self.Canmove`)))
  (cast `/Game/PlayerBP/Blueprints/FirstPersonCharacter` OtherActor)
  (if (`self.CanMove?`)
    (`KismetSystemLibrary.PrintString` "You've been killed en sah")))

(fn `UserConstructionScript`)