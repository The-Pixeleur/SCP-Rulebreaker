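; SCP-106 AI character that periodically materializes to hunt the player, then withdraws.
; Unless contained at BeginPlay, a short countdown triggers Appear, which teleports it in front of the player with animation and sounds, then starts the chase.
; ChasePlayer re-issues AI MoveTo on success or failure, while a long delay eventually halts it, teleports it to DebugSpawnZone and restarts the countdown.
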(event `StartCountdown`
  (`KismetSystemLibrary.Delay` 5.0)
  (`self.Appear`))

(event `self.ReceiveBeginPlay`
  (if (`self.Contained?`)
    _
    (elif (`self.Appeared?`)
      (`self.ChasePlayer`)
      (else
        (`self.StartCountdown`)))))

(event `ChasePlayer`
  (bind _returnvalue (`GameplayStatics.GetPlayerCharacter` 0))
  (`|ExecutionSequence`
    (:`then_0`
      (if (`self.Appeared?`)
        (`|AIMoveTo` self (`self.K2_GetActorLocation` _returnvalue) _returnvalue
          (:`then`
            (`KismetSystemLibrary.PrintString` "MOVE" true true (struct :`G` 0.804581 :`B` 1.0 :`A` 1.0)))
          (:`OnSuccess`
            (`self.ChasePlayer` :!label _label))
          (:`OnFail`
            (goto _label)))))
    (:`then_1`
      (if (`self.Appeared?`)
        (`KismetSystemLibrary.Delay` 101.5)
        (set `CharacterMovementComponent.MaxWalkSpeed` 0.0 (`self.CharacterMovement`))
        (`SkeletalMeshComponent.PlayAnimation` (`self.Mesh`) "/Game/AI/SCPs/106/Model3d/Reworked_106_Anim_106_2_skeleton_106_2_skeleton_106_2_skeleton_106_2_skeleton_106_2_skeleton_006.Reworked_106_Anim_106_2_skeleton_106_2_skeleton_106_2_skeleton_106_2_skeleton_106_2_skeleton_006" true)
        (`KismetSystemLibrary.Delay` 1.0)
        (`self.K2_TeleportTo` (`self.DebugSpawnZone`))
        (set `self.Appeared?` false)
        (`self.StartCountdown`)))))

(event `Appear`
  (bind _returnvalue (`GameplayStatics.GetPlayerCharacter` 0))
  (bind _mesh (`self.Mesh`))
  (bind _returnvalue_2 (`SceneComponent.K2_GetComponentLocation` _mesh))
  (if (not (`self.Appeared?`))
    (set `self.Appeared?` true)
    (set `CharacterMovementComponent.MaxWalkSpeed` 0.0 (`self.CharacterMovement`))
    (`self.K2_TeleportTo` (+ (`self.K2_GetActorLocation` _returnvalue) (* (`self.GetActorForwardVector` _returnvalue) 800.0)))
    (`SkeletalMeshComponent.PlayAnimation` _mesh "/Game/AI/SCPs/106/Model3d/Reworked_106_Anim_106_2_skeleton_106_2_skeleton_106_2_skeleton_106_2_skeleton_106_2_skeleton_003.Reworked_106_Anim_106_2_skeleton_106_2_skeleton_106_2_skeleton_106_2_skeleton_106_2_skeleton_003" false)
    (`GameplayStatics.SpawnSoundAttached` "/Game/AI/SCPs/106/SFX/106_Chase_Cue.106_Chase_Cue" _mesh "None" _returnvalue_2 (struct) "KeepRelativeOffset" false 1.0 1.0 0.0 null null)
    (`GameplayStatics.PlaySoundAtLocation` "/Game/AI/SCPs/106/SFX/Laugh106_Cue.Laugh106_Cue" _returnvalue_2 (struct) 1.0 1.0 0.0 null null null)
    (`KismetSystemLibrary.Delay` 6.0)
    (`SkeletalMeshComponent.PlayAnimation` (`self.Mesh`) "/Game/AI/SCPs/106/Model3d/Reworked_106_Anim_106_2_skeleton_106_2_skeleton_106_2_skeleton_106_2_skeleton_106_2_skeleton_007.Reworked_106_Anim_106_2_skeleton_106_2_skeleton_106_2_skeleton_106_2_skeleton_106_2_skeleton_007" true)
    (set `CharacterMovementComponent.MaxWalkSpeed` 200.0 (`self.CharacterMovement`))
    (`self.ChasePlayer`)))

(fn `UserConstructionScript`)