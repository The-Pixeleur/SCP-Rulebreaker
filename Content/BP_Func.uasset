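; BP_Func is a set of shared gameplay helpers for on-screen hints and surface-based walking sounds.
; Hints creates a UI_Hints widget with a title and description, plays its show animation and adds it to the viewport.
; WalingSound uses MovementCheking to confirm grounded movement, then traces downward and plays a sound chosen by physical-material surface type at the hit point.
; ShowSousTitre is an empty stub.
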(fn `Hints`
  (params (Titre :type Text) (Desc :type Text))
  (bind _returnvalue (`|CreateWidget` "/Game/UI/popus/UI_Hints.UI_Hints_C" null Titre Desc))
  (`UserWidget.PlayAnimation` _returnvalue (`/Game/UI/popus/UI_Hints.ShowAnim` _returnvalue) 0.0 1 "Forward" 1.0 false)
  (`UserWidget.AddToViewport` _returnvalue 0))

(fn `MovementCheking`
  (params (Target :type "NavMovementComponent Object Reference"))
  (returns (`Moving?` :type Boolean))
  (if (`NavMovementComponent.IsMovingOnGround` Target)
    (if (!= (`MovementComponent.Velocity` Target) (0.0 0.0 0.0) :`ErrorTolerance` 0.01)
      (return true))))

(fn `ShowSousTitre`)

(fn `WalingSound`
  (params (ModelToCheck :type "SceneComponent Object Reference") (ModelCharMov :type "NavMovementComponent Object Reference"))
  (locals (EnumWalkingMat :type Byte) (SoundMetal :type "SoundCue Object Reference" :default "SoundCue'/Game/Audio/Walking/Metal/Metal_Walk_Cue.Metal_Walk_Cue'") (SoundWood :type "SoundCue Object Reference") (SoundTile :type "SoundCue Object Reference" :default "SoundCue'/Game/Audio/Walking/Asphalt/Asphalt_Walk_Cue.Asphalt_Walk_Cue'") (SoundAsphalt :type "SoundCue Object Reference" :default "SoundCue'/Game/Audio/Walking/Asphalt/Asphalt_Walk_Cue.Asphalt_Walk_Cue'"))
  (bind _returnvalue (`SceneComponent.K2_GetComponentLocation` ModelToCheck))
  (bind _soundmetal (`local.SoundMetal`))
  (bind _soundasphalt (`local.SoundAsphalt`))
  (`/Engine/EditorBlueprintResources/StandardMacros.IsValid` ModelToCheck
    (:`Is Valid`
      (`/Engine/EditorBlueprintResources/StandardMacros.IsValid` ModelCharMov
        (:`Is Valid`
          (bind _moving_ (`self.MovementCheking` ModelCharMov))
          (if _moving_
            (bind _outhit (`KismetSystemLibrary.LineTraceSingle` null _returnvalue (+ _returnvalue (0.0 0.0 -150.0)) "TraceTypeQuery1" true))
            (bind (_bblockinghit _binitialoverlap _time _distance _location _impactpoint _normal _impactnormal _physmat) (`GameplayStatics.BreakHitResult` _outhit))
            (`/Engine/EditorBlueprintResources/StandardMacros.IsValid` _physmat
              (:`Is Valid`
                (`GameplayStatics.PlaySoundAtLocation` null (select `EPhysicalSurface` (`PhysicalMaterial.SurfaceType` _physmat) :`SurfaceType_Default` "/Game/Audio/Walking/Asphalt/Asphalt_Walk_Cue.Asphalt_Walk_Cue" :`SurfaceType1` (`local.SoundTile`) :`SurfaceType2` _soundmetal :`SurfaceType3` _soundasphalt :`SurfaceType4` _soundasphalt :`SurfaceType5` _soundmetal :`SurfaceType7` (`local.SoundWood`)) _impactpoint (struct) 2.0 1.0 0.0 "/Game/Audio/Attenuation/AlarmAttenuation.AlarmAttenuation" null null)))))))))