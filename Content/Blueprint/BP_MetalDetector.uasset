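; BP_MetalDetector is a metal detector actor that sets off an alarm when the first-person character enters its trigger box while it is activated.
; The overlap plays a sound, turns two spotlights red and starts a self-calling Light event that rotates the cylinder in small delayed steps.
; A retriggerable delay, timed slightly shorter than the sound, then blacks out the lights and stops the rotation.
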(event `self.Box.OnComponentBeginOverlap`
  (params (OverlappedComponent :type "PrimitiveComponent Object Reference") (OtherActor :type "Actor Object Reference") (OtherComp :type "PrimitiveComponent Object Reference") (OtherBodyIndex :type Integer) (bFromSweep :type Boolean) (SweepResult :type "HitResult Structure (by ref)"))
  (bind _sound (`self.Sound`))
  (if (`self.Activated?`)
    (cast `/Game/PlayerBP/Blueprints/FirstPersonCharacter` OtherActor)
    (`GameplayStatics.PlaySoundAtLocation` _sound (`SceneComponent.K2_GetComponentLocation` (`self.StaticMesh`)) (struct) 1.0 1.0 0.0 null null null)
    (`LightComponent.SetLightColor` (`self.SpotLight1`) (struct :`R` 1.0 :`A` 1.0) true)
    (`LightComponent.SetLightColor` (`self.SpotLight`) (struct :`R` 1.0 :`A` 1.0) true)
    (set `self.CanRotate` true)
    (`self.Light`)
    (`KismetSystemLibrary.RetriggerableDelay` (- (`SoundBase.Duration` _sound) 2.0))
    (`LightComponent.SetLightColor` (`self.SpotLight`) (struct :`A` 1.0) true)
    (`LightComponent.SetLightColor` (`self.SpotLight1`) (struct :`A` 1.0) true)
    (set `self.CanRotate` false)))

(event `Light`
  (if (`self.CanRotate`)
    (`KismetSystemLibrary.Delay` 0.025)
    (`SceneComponent.K2_AddLocalRotation` (`self.Cylinder`) (struct :`Yaw` 5.0) false false)
    (`self.Light`)))

(fn `UserConstructionScript`)