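; Big button Blueprint that spawns a batch of actors when its EvenementDuBouton event fires.
; The event loops over the Class array and spawns repeated copies of each class, with the repeat count driven by LastIndex.
; Each copy appears at a random point inside the bounds of the referenced Area's collision component.
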(event `self.EvenementDuBouton`
  (bind (_origin _boxextent) (`KismetSystemLibrary.GetComponentBounds` (`TriggerBase.CollisionComponent` (`self.Area`))))
  (for _array_element (`self.Class`)
    (for _ (range (+ (`self.Last Index`) 1))
      (`|SpawnActorFromClass` _array_element (`KismetMathLibrary.MakeTransform` (`KismetMathLibrary.RandomPointInBoundingBox` _origin _boxextent)) "Undefined" "OverrideRootScale" null null))))

(fn `UserConstructionScript`
  (`parent.UserConstructionScript`))