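; Base item actor that highlights itself when looked at and reports its item struct, stamped with its class, to the first-person character.
; Box overlap toggles Tick, which gates a camera line trace behind a facing dot-product check.
; A traced item gets custom-depth highlighting and fills the character's ItemInVisor.
; A self-repeating half-second delay loop moves the root to the mesh's location.
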(event `self.ReceiveBeginPlay`
  (bind (_itemtype_itemname _itemtype_itemimage _itemtype_itemtype) (break `/Game/PlayerBP/Blueprints/S_Item` (`self.ItemType`)))
  (set `self.ItemType` (make `/Game/PlayerBP/Blueprints/S_Item` _itemtype_itemname _itemtype_itemimage _itemtype_itemtype (`GameplayStatics.GetObjectClass` self)))
  (`self.FalseTime`))

(event `FalseTime`
  (bind _itemmesh (`self.ItemMesh`))
  (`/Engine/EditorBlueprintResources/StandardMacros.IsValid` _itemmesh
    (:`Is Valid`
      (`SceneComponent.K2_SetWorldLocation` (`self.DefaultSceneRoot`) (`SceneComponent.K2_GetComponentLocation` _itemmesh) false false))
    (:`Is Not Valid`
      _))
  (`KismetSystemLibrary.Delay` 0.5)
  (`self.FalseTime`))

(event `self.Box.OnComponentBeginOverlap`
  (params (OverlappedComponent :type "PrimitiveComponent Object Reference") (OtherActor :type "Actor Object Reference") (OtherComp :type "PrimitiveComponent Object Reference") (OtherBodyIndex :type Integer) (bFromSweep :type Boolean) (SweepResult :type "HitResult Structure (by ref)"))
  (bind _asfirst_person_character (cast `/Game/PlayerBP/Blueprints/FirstPersonCharacter` OtherActor))
  (set `self.As First Person Character` _asfirst_person_character)
  (`self.SetActorTickEnabled` true))

(event `self.Box.OnComponentEndOverlap`
  (params (OverlappedComponent :type "PrimitiveComponent Object Reference") (OtherActor :type "Actor Object Reference") (OtherComp :type "PrimitiveComponent Object Reference") (OtherBodyIndex :type Integer))
  (bind _asfirst_person_character (cast `/Game/PlayerBP/Blueprints/FirstPersonCharacter` OtherActor))
  (set `self.As First Person Character` _asfirst_person_character)
  (`self.SetActorTickEnabled` false)
  (`PrimitiveComponent.SetRenderCustomDepth` (`self.ItemMesh`) false))

(event `self.ReceiveTick`
  (params (DeltaSeconds :type "Float (single-precision)"))
  (bind _as_first_person_character (`self.As First Person Character`))
  (bind _item_meshref (`self.Item MeshRef`))
  (bind _as_first_person_character_2 (`self.As First Person Character`))
  (bind _firstpersoncamera (`/Game/PlayerBP/Blueprints/FirstPersonCharacter.FirstPersonCamera` _as_first_person_character_2))
  (bind _firstpersoncamera_2 (`/Game/PlayerBP/Blueprints/FirstPersonCharacter.FirstPersonCamera` (`self.As First Person Character`)))
  (bind _returnvalue (`SceneComponent.K2_GetComponentLocation` _firstpersoncamera_2))
  (if (>= (* (`KismetMathLibrary.Dot_VectorVector` (`KismetMathLibrary.GetForwardVector` (`KismetMathLibrary.FindLookAtRotation` (`SceneComponent.K2_GetComponentLocation` (`self.ItemMesh`)) (`SceneComponent.K2_GetComponentLocation` _firstpersoncamera))) (`SceneComponent.GetForwardVector` _firstpersoncamera)) -10.0) 9.0)
    (bind _outhit (`KismetSystemLibrary.LineTraceSingle` _returnvalue (+ _returnvalue (* (`SceneComponent.GetForwardVector` _firstpersoncamera_2) 50000.0)) "TraceTypeQuery1" true (`|MakeArray` (`/Game/PlayerBP/Blueprints/FirstPersonCharacter.WeaponRef` _as_first_person_character_2) :!type "Actor Object Reference") "None" false))
    (bind _asbp_item_master (cast `/Game/Blueprint/Object/BP_Item_Master` (`.HitActor` (`GameplayStatics.BreakHitResult` _outhit)))
      (:`then`
        (bind _itemmesh (`/Game/Blueprint/Object/BP_Item_Master.ItemMesh` _asbp_item_master))
        (if (!= _item_meshref _itemmesh)
          (`/Engine/EditorBlueprintResources/StandardMacros.IsValid` _item_meshref
            (:`Is Valid`
              (`PrimitiveComponent.SetRenderCustomDepth` _item_meshref false))
            (:`Is Not Valid`
              _)))
        (bind _output_get (set `self.Item MeshRef` _itemmesh))
        (`PrimitiveComponent.SetRenderCustomDepth` _output_get true)
        (`/Engine/EditorBlueprintResources/StandardMacros.IsValid` _as_first_person_character
          (:`Is Valid`
            (set `/Game/PlayerBP/Blueprints/FirstPersonCharacter.itemInVisor` (`/Game/Blueprint/Object/BP_Item_Master.ItemType` _asbp_item_master) _as_first_person_character))))
      (:`CastFailed`
        (`/Engine/EditorBlueprintResources/StandardMacros.IsValid` _item_meshref
          (:`Is Valid`
            (`PrimitiveComponent.SetRenderCustomDepth` _item_meshref false)))))
    (else
      (`self.DisableInput` (`GameplayStatics.GetPlayerController` 0)))))

(event `Effect`)

(fn `UserConstructionScript`)