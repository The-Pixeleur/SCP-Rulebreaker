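; BP_Item_SCP2022 is an SCP item Blueprint whose effect toggles a status flag on the player.
; Its Effect event casts the first player pawn to FirstPersonCharacter and flips HasSCP714, a flag named after SCP-714 rather than SCP-2022.
; The BeginPlay, overlap and Tick events are disabled stubs, and the construction script only calls its parent.
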(event `self.Effect`
  (bind _asfirst_person_character (cast `/Game/PlayerBP/Blueprints/FirstPersonCharacter` (`GameplayStatics.GetPlayerPawn` 0)))
  (if (`/Game/PlayerBP/Blueprints/FirstPersonCharacter.HasSCP714?` _asfirst_person_character)
    (set `/Game/PlayerBP/Blueprints/FirstPersonCharacter.HasSCP714?` false _asfirst_person_character)
    (else
      (set `/Game/PlayerBP/Blueprints/FirstPersonCharacter.HasSCP714?` true _asfirst_person_character))))

(fn `UserConstructionScript`
  (`parent.UserConstructionScript`))