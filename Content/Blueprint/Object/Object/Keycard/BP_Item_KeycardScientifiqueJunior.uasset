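; Junior scientist keycard item that the player can hold in hand to gain its opening level.
; Its Effect event toggles on the first-person character's hands-occupied flag.
; With empty hands, it copies its opening level to the character and shows a second-hand keycard using its own mesh's front material.
; If something is already held, it resets that level, clears the flag and removes the left-hand item.
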(event `self.Effect`
  (bind _asfirst_person_character (cast `/Game/PlayerBP/Blueprints/FirstPersonCharacter` (`GameplayStatics.GetPlayerPawn` 0)))
  (if (`/Game/PlayerBP/Blueprints/FirstPersonCharacter.GetSomethinInHands?` _asfirst_person_character)
    (set `/Game/PlayerBP/Blueprints/FirstPersonCharacter.CurrentOpeninLevel` 0 _asfirst_person_character)
    (set `/Game/PlayerBP/Blueprints/FirstPersonCharacter.GetSomethinInHands?` false _asfirst_person_character)
    (`/Game/PlayerBP/Blueprints/FirstPersonCharacter.RemoveLefthands` _asfirst_person_character)
    (else
      (set `/Game/PlayerBP/Blueprints/FirstPersonCharacter.CurrentOpeninLevel` (`self.Current Openin Level`) _asfirst_person_character)
      (set `/Game/PlayerBP/Blueprints/FirstPersonCharacter.GetSomethinInHands?` true _asfirst_person_character)
      (`/Game/PlayerBP/Blueprints/FirstPersonCharacter.SetSecondHandsKeycard` _asfirst_person_character "/Game/Blueprint/Object/BP_keycardref.BP_keycardref_C" (`PrimitiveComponent.GetMaterial` (`self.ItemMesh`) 1)))))

(fn `UserConstructionScript`
  (`parent.UserConstructionScript`))