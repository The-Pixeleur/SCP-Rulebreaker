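; BP_Item_Ammo556mm is an item that gives the player 5.56x45mm ammunition.
; Its Effect event casts player pawn 0 to FirstPersonCharacter, increases that character's 556x45mmCount by a fixed amount, then sets ShouldBeDestroyed.
; If the cast fails, nothing changes; the other event nodes are disabled and the construction script only calls the parent.
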(event `self.Effect`
  (bind _asfirst_person_character (cast `/Game/PlayerBP/Blueprints/FirstPersonCharacter` (`GameplayStatics.GetPlayerPawn` 0)))
  (set `/Game/PlayerBP/Blueprints/FirstPersonCharacter.556x45mm_count` (+ (`/Game/PlayerBP/Blueprints/FirstPersonCharacter.556x45mm_count` _asfirst_person_character) 25) _asfirst_person_character)
  (set `self.ShouldBeDestroyed?` true))

(fn `UserConstructionScript`
  (`parent.UserConstructionScript`))