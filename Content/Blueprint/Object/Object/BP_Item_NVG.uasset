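; Night vision goggles item that toggles the player's NVG state when its Effect event runs.
; Effect casts the player pawn to FirstPersonCharacter and flips its NVG flag.
; Switching NVG on also clears both SCRAMBLER flags and calls the character's 096Check, so the two devices are not active together.
; It sets ShouldBeDestroyed to false after toggling, marking the item as reusable.
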(event `self.Effect`
  (bind _asfirst_person_character (cast `/Game/PlayerBP/Blueprints/FirstPersonCharacter` (`GameplayStatics.GetPlayerPawn` 0)))
  (if (`/Game/PlayerBP/Blueprints/FirstPersonCharacter.NVG?` _asfirst_person_character)
    (set `/Game/PlayerBP/Blueprints/FirstPersonCharacter.NVG?` false _asfirst_person_character)
    (else
      (set `/Game/PlayerBP/Blueprints/FirstPersonCharacter.NVG?` true _asfirst_person_character)
      (set `/Game/PlayerBP/Blueprints/FirstPersonCharacter.SCRAMBLER?` false _asfirst_person_character)
      (set `/Game/PlayerBP/Blueprints/FirstPersonCharacter.SCRAMBLESactivated?` false _asfirst_person_character)
      (`/Game/PlayerBP/Blueprints/FirstPersonCharacter.096Check` _asfirst_person_character)))
  (set `self.ShouldBeDestroyed?` false))

(fn `UserConstructionScript`
  (`parent.UserConstructionScript`))