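; Master weapon pickup that displays a physics-simulated weapon and lets the player swap it for the held one.
; It spawns the weapon and attachments from NewWeaponStruct, moving its GeometryCollection to the weapon body twice a second.
; Box overlap shows a stats widget and enables Tick, which allows input only while the camera faces the weapon.
; E spawns a replacement pickup holding the player's weapon data, hands over the stored weapon, then destroys itself.
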(event `FalseTime`
  (bind _weapon (`self.Weapon`))
  (`/Engine/EditorBlueprintResources/StandardMacros.IsValid` _weapon
    (:`Is Valid`
      (`SceneComponent.K2_SetWorldLocation` (`self.GeometryCollection`) (`SceneComponent.K2_GetComponentLocation` (`/Game/Blueprint/Weapon/BP_Weapon_Master.WeaponBody` _weapon)) false false))
    (:`Is Not Valid`
      _))
  (`KismetSystemLibrary.Delay` 0.5)
  (`self.FalseTime`))

(event `self.ReceiveBeginPlay`
  (`self.AddWeapon`)
  (`self.FalseTime`))

(event `AddWeapon`
  (bind (_ammocurrent _weaponcurrent _topattachment _sideattachment _bottomattachment _tipattachment _topattachment_transform _sideattachment_transform _bottomattachment_transform _tipattachment_transform) (break `/Game/Blueprint/Object/Weapon/S_WeaponGrab` (`self.NewWeaponStruct`)))
  (bind _returnvalue (`|SpawnActorFromClass` _weaponcurrent (`SceneComponent.K2_GetComponentToWorld` (`self.GunBody`)) "Undefined" "OverrideRootScale" null null))
  (bind _output_get (set `self.Weapon` _returnvalue))
  (`/Engine/EditorBlueprintResources/StandardMacros.IsValid` _output_get
    (:`Is Valid`
      (`PrimitiveComponent.SetSimulatePhysics` (`/Game/Blueprint/Weapon/BP_Weapon_Master.WeaponBody` _output_get) true)
      (`|ExecutionSequence`
        (:`then_0`
          (`/Engine/EditorBlueprintResources/StandardMacros.IsValid` _topattachment
            (:`Is Valid`
              (`/Game/Blueprint/Weapon/BP_Weapon_Master.SetAttachment` _output_get (`/Game/Blueprint/Weapon/BP_Weapon_Master.TopAttachment` _output_get) _topattachment _topattachment_transform))))
        (:`then_1`
          (`/Engine/EditorBlueprintResources/StandardMacros.IsValid` _sideattachment
            (:`Is Valid`
              (`/Game/Blueprint/Weapon/BP_Weapon_Master.SetAttachment` _output_get (`/Game/Blueprint/Weapon/BP_Weapon_Master.SideAttachment` _output_get) _sideattachment _sideattachment_transform))))
        (:`then_2`
          (`/Engine/EditorBlueprintResources/StandardMacros.IsValid` _tipattachment
            (:`Is Valid`
              (`/Game/Blueprint/Weapon/BP_Weapon_Master.SetAttachment` _output_get (`/Game/Blueprint/Weapon/BP_Weapon_Master.TipAttachment` _output_get) _tipattachment _tipattachment_transform))))
        (:`then_3`
          (`/Engine/EditorBlueprintResources/StandardMacros.IsValid` _bottomattachment
            (:`Is Valid`
              (`/Game/Blueprint/Weapon/BP_Weapon_Master.SetAttachment` _output_get (`/Game/Blueprint/Weapon/BP_Weapon_Master.BottomAttachment` _output_get) _bottomattachment _bottomattachment_transform))))))))

(event `self.ReceiveTick`
  (params (DeltaSeconds :type "Float (single-precision)"))
  (bind _returnvalue (`GameplayStatics.GetPlayerController` 0))
  (bind _firstpersoncamera (`/Game/PlayerBP/Blueprints/FirstPersonCharacter.FirstPersonCamera` (`self.As First Person Character`)))
  (if (>= (* (`KismetMathLibrary.Dot_VectorVector` (`KismetMathLibrary.GetForwardVector` (`KismetMathLibrary.FindLookAtRotation` (`SceneComponent.RelativeLocation` (`/Game/Blueprint/Weapon/BP_Weapon_Master.WeaponBody` (`self.Weapon`))) (`SceneComponent.K2_GetComponentLocation` _firstpersoncamera))) (`SceneComponent.GetForwardVector` _firstpersoncamera)) -10.0) 9.0)
    (`self.EnableInput` _returnvalue)
    (else
      (`self.DisableInput` _returnvalue))))

(event `self.Box.OnComponentBeginOverlap`
  (params (OverlappedComponent :type "PrimitiveComponent Object Reference") (OtherActor :type "Actor Object Reference") (OtherComp :type "PrimitiveComponent Object Reference") (OtherBodyIndex :type Integer) (bFromSweep :type Boolean) (SweepResult :type "HitResult Structure (by ref)"))
  (bind _weapon (`self.Weapon`))
  (bind _asfirst_person_character (cast `/Game/PlayerBP/Blueprints/FirstPersonCharacter` OtherActor))
  (set `self.As First Person Character` _asfirst_person_character)
  (`self.SetActorTickEnabled` true)
  (`/Engine/EditorBlueprintResources/StandardMacros.IsValid` _weapon
    (:`Is Valid`
      (bind _output_get (set `self.caliber` (`/Game/Blueprint/Weapon/BP_Weapon_Master.Caliber` _weapon)))
      (bind _returnvalue (`|CreateWidget` "/Game/UI/Weapon/widget_WeaponStat.widget_WeaponStat_C" null (`/Game/Blueprint/Weapon/BP_Weapon_Master.WeaponDisplayName` _weapon) (`KismetTextLibrary.Conv_StringToText` (`|GetEnumeratorNameAsString` _output_get)) (`.AmmoCurrent_6_2DE6CD794AA20479A97BB18939774225` (break `/Game/Blueprint/Object/Weapon/S_WeaponGrab` (`self.NewWeaponStruct`))) (`/Game/Blueprint/Weapon/BP_Weapon_Master.AmmoMax` _weapon)))
      (`WidgetComponent.SetWidget` (`self.Widget`) _returnvalue))))

(event `self.Box.OnComponentEndOverlap`
  (params (OverlappedComponent :type "PrimitiveComponent Object Reference") (OtherActor :type "Actor Object Reference") (OtherComp :type "PrimitiveComponent Object Reference") (OtherBodyIndex :type Integer))
  (cast `/Game/PlayerBP/Blueprints/FirstPersonCharacter` OtherActor)
  (`self.SetActorTickEnabled` false)
  (`WidgetComponent.SetWidget` (`self.Widget`) null)
  (`self.DisableInput` (`GameplayStatics.GetPlayerController` 0)))

(event `Key|E`
  (params (Key :type "Key Structure"))
  (bind _weapon (`self.Weapon`))
  (bind _as_first_person_character (`self.As First Person Character`))
  (bind _weaponref (`/Game/PlayerBP/Blueprints/FirstPersonCharacter.WeaponRef` _as_first_person_character))
  (bind _topattachment (`/Game/Blueprint/Weapon/BP_Weapon_Master.TopAttachment` _weaponref))
  (bind _sideattachment (`/Game/Blueprint/Weapon/BP_Weapon_Master.SideAttachment` _weaponref))
  (bind _bottomattachment (`/Game/Blueprint/Weapon/BP_Weapon_Master.BottomAttachment` _weaponref))
  (bind _tipattachment (`/Game/Blueprint/Weapon/BP_Weapon_Master.TipAttachment` _weaponref))
  (:`Pressed`
    (for _array_element (`PrimitiveComponent.GetOverlappingActors` (`self.Box`) "/Game/PlayerBP/Blueprints/FirstPersonCharacter.FirstPersonCharacter_C")
      (bind _asfirst_person_character (cast `/Game/PlayerBP/Blueprints/FirstPersonCharacter` _array_element))
      (set `self.As First Person Character` _asfirst_person_character))
    (`/Game/Blueprint/Weapon/BP_Weapon_Master.HandToBottom` _weaponref)
    (`KismetSystemLibrary.Delay` 0.3)
    (bind _returnvalue (`|SpawnActorFromClass` "BP_WeaponToGrab_Master_C" (`self.GetTransform`) "Undefined" "OverrideRootScale" null null))
    (set `self.OldWeaponStruct` (`self.NewWeaponStruct`))
    (set `/Game/Blueprint/Object/Weapon/BP_WeaponToGrab_Master.NewWeaponStruct` (make `/Game/Blueprint/Object/Weapon/S_WeaponGrab` (`/Game/Blueprint/Weapon/BP_Weapon_Master.AmmoCurrent` _weaponref) (`GameplayStatics.GetObjectClass` _weaponref) (`StaticMeshComponent.StaticMesh` _topattachment) (`StaticMeshComponent.StaticMesh` _sideattachment) (`StaticMeshComponent.StaticMesh` _bottomattachment) (`StaticMeshComponent.StaticMesh` _tipattachment) (`SceneComponent.GetRelativeTransform` _topattachment) (`SceneComponent.GetRelativeTransform` _sideattachment) (`SceneComponent.GetRelativeTransform` _bottomattachment) (`SceneComponent.GetRelativeTransform` _tipattachment)) _returnvalue)
    (`/Game/PlayerBP/Blueprints/FirstPersonCharacter.NewWeapon` _as_first_person_character (`self.OldWeaponStruct`))
    (`self.AddWeapon` _returnvalue)
    (`/Game/Blueprint/Weapon/BP_Weapon_Master.HandBackToNormal` _weaponref)
    (`KismetSystemLibrary.PrintString` (`KismetStringLibrary.Concat_StrStr` "Vous avez récuperer un " (`KismetTextLibrary.Conv_TextToString` (`/Game/Blueprint/Weapon/BP_Weapon_Master.WeaponDisplayName` _weaponref))))
    (`SceneComponent.K2_DetachFromComponent` (`self.GeometryCollection`) "KeepWorld" "KeepWorld" "KeepWorld" true)
    (while (`KismetSystemLibrary.IsValid` _weapon)
      (`self.K2_DestroyActor` _weapon))
    (`self.K2_DestroyActor`)))

(fn `UserConstructionScript`)