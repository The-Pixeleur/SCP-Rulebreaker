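; BP_PhoneBen is an interactable phone prop that plays a Talking Ben sound at its mesh when the player presses Use while looking at it.
; A Box overlap with the first-person character toggles Tick, which runs a view-direction dot check and then a camera line trace.
; A trace hit on the actor turns on a custom depth highlight on the mesh (named ScrantonRealityAnchor) and enables input for the Use action.
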(event `self.Box.OnComponentBeginOverlap`
  (params (OverlappedComponent :type "PrimitiveComponent Object Reference") (OtherActor :type "Actor Object Reference") (OtherComp :type "PrimitiveComponent Object Reference") (OtherBodyIndex :type Integer) (bFromSweep :type Boolean) (SweepResult :type "HitResult Structure (by ref)"))
  (bind _asfirst_person_character (cast `/Game/PlayerBP/Blueprints/FirstPersonCharacter` OtherActor))
  (set `self.As First Person Character` _asfirst_person_character)
  (`self.SetActorTickEnabled` true))

(event `self.Box.OnComponentEndOverlap`
  (params (OverlappedComponent :type "PrimitiveComponent Object Reference") (OtherActor :type "Actor Object Reference") (OtherComp :type "PrimitiveComponent Object Reference") (OtherBodyIndex :type Integer))
  (bind _asfirst_person_character (cast `/Game/PlayerBP/Blueprints/FirstPersonCharacter` OtherActor))
  (set `self.As First Person Character` _asfirst_person_character)
  (`self.SetActorTickEnabled` false)
  (`PrimitiveComponent.SetRenderCustomDepth` (`self.ScrantonRealityAnchor`) false))

(event `self.ReceiveTick`
  (params (DeltaSeconds :type "Float (single-precision)"))
  (bind _returnvalue (`GameplayStatics.GetPlayerController` 0))
  (bind _scrantonrealityanchor (`self.ScrantonRealityAnchor`))
  (bind _as_first_person_character (`self.As First Person Character`))
  (bind _firstpersoncamera (`/Game/PlayerBP/Blueprints/FirstPersonCharacter.FirstPersonCamera` _as_first_person_character))
  (bind _firstpersoncamera_2 (`/Game/PlayerBP/Blueprints/FirstPersonCharacter.FirstPersonCamera` (`self.As First Person Character`)))
  (bind _returnvalue_2 (`SceneComponent.K2_GetComponentLocation` _firstpersoncamera_2))
  (if (>= (* (`KismetMathLibrary.Dot_VectorVector` (`KismetMathLibrary.GetForwardVector` (`KismetMathLibrary.FindLookAtRotation` (`SceneComponent.K2_GetComponentLocation` (`self.ScrantonRealityAnchor`)) (`SceneComponent.K2_GetComponentLocation` _firstpersoncamera))) (`SceneComponent.GetForwardVector` _firstpersoncamera)) -10.0) 9.0)
    (bind _outhit (`KismetSystemLibrary.LineTraceSingle` _returnvalue_2 (+ _returnvalue_2 (* (`SceneComponent.GetForwardVector` _firstpersoncamera_2) 50000.0)) "TraceTypeQuery1" true (`|MakeArray` (`/Game/PlayerBP/Blueprints/FirstPersonCharacter.WeaponRef` _as_first_person_character) _as_first_person_character (`GameplayStatics.GetPlayerCharacter` 0) (`GameplayStatics.GetPlayerPawn` 0) :!type "Actor Object Reference") "None" false))
    (if (== (`.HitActor` (`GameplayStatics.BreakHitResult` _outhit)) self)
      (`PrimitiveComponent.SetRenderCustomDepth` _scrantonrealityanchor true)
      (`self.EnableInput` _returnvalue)
      (else
        (`PrimitiveComponent.SetRenderCustomDepth` _scrantonrealityanchor false)
        (`self.DisableInput` _returnvalue)))
    (else
      (`self.DisableInput` (`GameplayStatics.GetPlayerController` 0)))))

(event `InputAction|Use`
  (params (Key :type "Key Structure"))
  (:`Pressed`
    (`GameplayStatics.PlaySoundAtLocation` "/Game/Audio/Meme/SoundEffect_TalkingBenPhone.SoundEffect_TalkingBenPhone" (`SceneComponent.K2_GetComponentLocation` (`self.ScrantonRealityAnchor`)) (struct) 2.5 1.0 0.0 "/Game/BallisticsVFX/SFX/Attentuations/ImpactsAttenuation.ImpactsAttenuation" null null)))

(fn `UserConstructionScript`)