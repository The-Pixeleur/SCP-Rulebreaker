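; Keycard-locked sliding door that the player opens and closes with Use, and that SCP-173 opens automatically.
; An overlap box enables input for the player, whose card level is checked against Levelneeded, while SCP-173 bypasses the check.
; A timeline lerps the door between closed and open positions, reversing to close.
; CheckKeycard plays granted or denied sounds and briefly swaps both readers' screen materials, with denial also printing a French debug message.
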(event `SetkeycardBase`
  (`PrimitiveComponent.SetMaterial` (`self.KeycardReader2`) 1 "/Game/Meshes/Props/KeycardReader/HE_ControlScreenLOCK.HE_ControlScreenLOCK")
  (`PrimitiveComponent.SetMaterial` (`self.KeycardReader1`) 1 "/Game/Meshes/Props/KeycardReader/HE_ControlScreenLOCK.HE_ControlScreenLOCK"))

(event `SetGood`
  (`PrimitiveComponent.SetMaterial` (`self.KeycardReader2`) 1 "/Game/Meshes/Props/KeycardReader/HE_ControlScreenGOOD.HE_ControlScreenGOOD")
  (`PrimitiveComponent.SetMaterial` (`self.KeycardReader1`) 1 "/Game/Meshes/Props/KeycardReader/HE_ControlScreenGOOD.HE_ControlScreenGOOD")
  (`KismetSystemLibrary.Delay` 1.2)
  (`self.SetkeycardBase`))

(event `SetBad`
  (`PrimitiveComponent.SetMaterial` (`self.KeycardReader2`) 1 "/Game/Meshes/Props/KeycardReader/HE_ControlScreenWRONG.HE_ControlScreenWRONG")
  (`PrimitiveComponent.SetMaterial` (`self.KeycardReader1`) 1 "/Game/Meshes/Props/KeycardReader/HE_ControlScreenWRONG.HE_ControlScreenWRONG")
  (`KismetSystemLibrary.Delay` 1.2)
  (`self.SetkeycardBase`))

(event `self.Box.OnComponentBeginOverlap`
  (params (OverlappedComponent :type "PrimitiveComponent Object Reference") (OtherActor :type "Actor Object Reference") (OtherComp :type "PrimitiveComponent Object Reference") (OtherBodyIndex :type Integer) (bFromSweep :type Boolean) (SweepResult :type "HitResult Structure (by ref)"))
  (cast `/Game/PlayerBP/Blueprints/FirstPersonCharacter` OtherActor
    (:`then`
      (`self.EnableInput` (`GameplayStatics.GetPlayerController` 0)))
    (:`CastFailed`
      (cast `/Game/AI/SCPs/173/BP_SCP-173` OtherActor)
      (`self.OpenDoor`))))

(event `self.Box.OnComponentEndOverlap`
  (params (OverlappedComponent :type "PrimitiveComponent Object Reference") (OtherActor :type "Actor Object Reference") (OtherComp :type "PrimitiveComponent Object Reference") (OtherBodyIndex :type Integer))
  (cast `/Game/PlayerBP/Blueprints/FirstPersonCharacter` OtherActor
    (:`then`
      (`self.DisableInput` (`GameplayStatics.GetPlayerController` 0)))
    (:`CastFailed`
      (cast `/Game/AI/SCPs/173/BP_SCP-173` OtherActor)
      (`self.CloseDoor`))))

(event `OpenDoor`
  (set `self.Open?` true :!label _label)
  (`self.CheckKeycard` true)
  (bind (_direction _newtrack_0) (`Timeline|Door` :!label _label_2)
    (:`Update`
      (`SceneComponent.K2_SetRelativeLocation` (`self.Cube`) (`KismetMathLibrary.VLerp` (`self.DoorPosClosed`) (`self.DoorPosOpen`) _newtrack_0) false false))))

(event `InputAction|Use`
  (params (Key :type "Key Structure"))
  (bind _levelneeded (`self.Levelneeded`))
  (:`Pressed`
    (bind _asfirst_person_character (cast `/Game/PlayerBP/Blueprints/FirstPersonCharacter` (`GameplayStatics.GetPlayerPawn` 0)))
    (bind _currentopeninlevel (`/Game/PlayerBP/Blueprints/FirstPersonCharacter.CurrentOpeninLevel` _asfirst_person_character))
    (if (>= _currentopeninlevel _levelneeded)
      (if (`self.Open?`)
        (set `self.Open?` false :!label _label_3)
        (`self.CheckKeycard` true)
        (goto _label_2 :!via `Reverse`)
        (else
          (goto _label)))
      (else
        (`KismetSystemLibrary.PrintString` (`KismetStringLibrary.Concat_StrStr` "Prends une carte niveau " (`KismetStringLibrary.Conv_IntToString` _levelneeded) " putain de con de merde" " \n" "Alors que le tié lvl : " (`KismetStringLibrary.Conv_IntToString` _currentopeninlevel)))
        (`self.CheckKeycard` false)))))

(event `CloseDoor`
  (goto _label_3))

(fn `CheckKeycard`
  (params (`CouldOpen?` :type Boolean))
  (bind _returnvalue (`SceneComponent.K2_GetComponentLocation` (`self.KeycardReader2`)))
  (bind _returnvalue_2 (`SceneComponent.K2_GetComponentLocation` (`self.KeycardReader1`)))
  (if `CouldOpen?`
    (`self.SetGood`)
    (`GameplayStatics.PlaySoundAtLocation` "/Game/Audio/Object/Button/KeyCardOpen_Cue.KeyCardOpen_Cue" _returnvalue (struct) 1.0 1.0 0.35 null null null)
    (`GameplayStatics.PlaySoundAtLocation` "/Game/Audio/Object/Button/KeyCardOpen_Cue.KeyCardOpen_Cue" _returnvalue_2 (struct) 1.0 1.0 0.35 null null null)
    (else
      (`self.SetBad`)
      (`GameplayStatics.PlaySoundAtLocation` "/Game/Audio/Object/Button/KeyCardDenied_Cue.KeyCardDenied_Cue" _returnvalue (struct) 1.0 1.0 0.0 null null null)
      (`GameplayStatics.PlaySoundAtLocation` "/Game/Audio/Object/Button/KeyCardDenied_Cue.KeyCardDenied_Cue" _returnvalue_2 (struct) 1.0 1.0 0.0 null null null))))

(fn `UserConstructionScript`)