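; BP_KeycardReader is a keycard reader for doors that shows locked, accepted or rejected states on its screen.
; SetGood and SetBad swap the screen material slot on both static meshes, then restore the locked material through SetkeycardBase after a short delay.
; It holds only this visual feedback, with no card validation or door logic in its graphs.
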(event `SetkeycardBase`
  (`PrimitiveComponent.SetMaterial` (`self.StaticMesh`) 1 "/Game/Meshes/Props/KeycardReader/HE_ControlScreenLOCK.HE_ControlScreenLOCK")
  (`PrimitiveComponent.SetMaterial` (`self.StaticMesh1`) 1 "/Game/Meshes/Props/KeycardReader/HE_ControlScreenLOCK.HE_ControlScreenLOCK"))

(event `SetGood`
  (`PrimitiveComponent.SetMaterial` (`self.StaticMesh`) 1 "/Game/Meshes/Props/KeycardReader/HE_ControlScreenGOOD.HE_ControlScreenGOOD")
  (`PrimitiveComponent.SetMaterial` (`self.StaticMesh1`) 1 "/Game/Meshes/Props/KeycardReader/HE_ControlScreenGOOD.HE_ControlScreenGOOD")
  (`KismetSystemLibrary.Delay` 1.2)
  (`self.SetkeycardBase`))

(event `SetBad`
  (`PrimitiveComponent.SetMaterial` (`self.StaticMesh`) 1 "/Game/Meshes/Props/KeycardReader/HE_ControlScreenWRONG.HE_ControlScreenWRONG")
  (`PrimitiveComponent.SetMaterial` (`self.StaticMesh1`) 1 "/Game/Meshes/Props/KeycardReader/HE_ControlScreenWRONG.HE_ControlScreenWRONG")
  (`KismetSystemLibrary.Delay` 1.2)
  (`self.SetkeycardBase`))

(fn `UserConstructionScript`)