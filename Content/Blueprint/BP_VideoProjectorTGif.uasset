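; An interactable video projector that the player switches on and off with the Use input, toggling its spotlight and looping cue after a button sound and short delay.
; A trigger box enables Tick while the first-person character is inside.
; Tick combines a camera-facing dot product with a line trace to highlight the projector via custom depth and enable input.
; Tick also randomizes the lit spotlight's intensity, producing projector flicker.
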(event `self.ReceiveBeginPlay`
  (if (not (!= (`LightComponentBase.Intensity` (`self.SpotLight`)) 0.0))
    (`AudioComponent.Stop` (`self.videoProjector_Cue`))))

(event `self.Box.OnComponentBeginOverlap`
  (params (OverlappedComponent :type "PrimitiveComponent Object Reference") (OtherActor :type "Actor Object Reference") (OtherComp :type "PrimitiveComponent Object Reference") (OtherBodyIndex :type Integer) (bFromSweep :type Boolean) (SweepResult :type "HitResult Structure (by ref)"))
  (bind _asfirst_person_character (cast `/Game/PlayerBP/Blueprints/FirstPersonCharacter` OtherActor))
  (set `self.As First Person Character` _asfirst_person_character)
  (`self.SetActorTickEnabled` true))

(event `self.Box.OnComponentEndOverlap`
  (params (OverlappedComponent :type "PrimitiveComponent Object Reference") (OtherActor :type "Actor Object Reference") (OtherComp :type "PrimitiveComponent Object Reference") (OtherBodyIndex :type Integer))
  (bind _asfirst_person_character (cast `/Game/PlayerBP/Blueprints/FirstPersonCharacter` OtherActor))
  (set `self.As First Person Character` _asfirst_person_character)
  (`self.SetActorTickEnabled` false)
  (`PrimitiveComponent.SetRenderCustomDepth` (`self.Cube`) false))

(event `self.ReceiveTick`
  (params (DeltaSeconds :type "Float (single-precision)"))
  (bind _returnvalue (`GameplayStatics.GetPlayerController` 0))
  (bind _as_first_person_character (`self.As First Person Character`))
  (bind _cube (`self.Cube`))
  (bind _firstpersoncamera (`/Game/PlayerBP/Blueprints/FirstPersonCharacter.FirstPersonCamera` _as_first_person_character))
  (bind _firstpersoncamera_2 (`/Game/PlayerBP/Blueprints/FirstPersonCharacter.FirstPersonCamera` (`self.As First Person Character`)))
  (bind _returnvalue_2 (`SceneComponent.K2_GetComponentLocation` _firstpersoncamera_2))
  (`|ExecutionSequence`
    (:`then_0`
      (if (>= (* (`KismetMathLibrary.Dot_VectorVector` (`KismetMathLibrary.GetForwardVector` (`KismetMathLibrary.FindLookAtRotation` (`SceneComponent.K2_GetComponentLocation` (`self.Cube`)) (`SceneComponent.K2_GetComponentLocation` _firstpersoncamera))) (`SceneComponent.GetForwardVector` _firstpersoncamera)) -10.0) 9.0)
        (bind _outhit (`KismetSystemLibrary.LineTraceSingle` _returnvalue_2 (+ _returnvalue_2 (* (`SceneComponent.GetForwardVector` _firstpersoncamera_2) 50000.0)) "TraceTypeQuery1" true (`|MakeArray` (`/Game/PlayerBP/Blueprints/FirstPersonCharacter.WeaponRef` _as_first_person_character) :!type "Actor Object Reference") "None" false))
        (if (== (`.HitActor` (`GameplayStatics.BreakHitResult` _outhit)) self)
          (`PrimitiveComponent.SetRenderCustomDepth` _cube true)
          (`self.EnableInput` _returnvalue)
          (else
            (`PrimitiveComponent.SetRenderCustomDepth` _cube false)
            (`self.DisableInput` _returnvalue)))
        (else
          (`self.DisableInput` (`GameplayStatics.GetPlayerController` 0)))))
    (:`then_1`
      (if (!= (`LightComponentBase.Intensity` (`self.SpotLight`)) 0.0)
        (`LightComponent.SetIntensity` (`self.SpotLight`) (`KismetMathLibrary.RandomFloatInRange` 1000.0 30000.0))))))

(event `ToggleWorking`
  (bind _spotlight (`self.SpotLight`))
  (bind _videoprojector_cue (`self.videoProjector_Cue`))
  (if (!= (`LightComponentBase.Intensity` _spotlight) 0.0) :!label _label
    (`LightComponent.SetIntensity` _spotlight 0.0)
    (`AudioComponent.Stop` _videoprojector_cue)
    (else
      (`LightComponent.SetIntensity` _spotlight 25000.0)
      (`AudioComponent.Play` _videoprojector_cue 0.0))))

(event `InputAction|Use`
  (params (Key :type "Key Structure"))
  (:`Pressed`
    (`GameplayStatics.PlaySoundAtLocation` "/Game/Audio/Object/VideoPorjector/projectorButton_Cue.projectorButton_Cue" (`SceneComponent.K2_GetComponentLocation` (`self.Cube`)) (struct) 1.0 1.0 0.385 null null null)
    (`KismetSystemLibrary.Delay` 0.2)
    (goto _label)))

(fn `UserConstructionScript`)