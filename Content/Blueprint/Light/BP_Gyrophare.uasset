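; BP_Gyrophare is a rotating emergency beacon light with an alarm sound that can be broken.
; On BeginPlay it starts Light, a self-calling event that rotates the Cube by a small yaw step after each short delay while CanRotate is true.
; The Breaking event clears CanRotate, stops the alarm audio and sets the SpotLight color to black.
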(event `self.ReceiveBeginPlay`
  (set `self.CanRotate` true)
  (`self.Light`))

(event `Light`
  (if (`self.CanRotate`)
    (`KismetSystemLibrary.Delay` 0.025)
    (`SceneComponent.K2_AddLocalRotation` (`self.Cube`) (struct :`Yaw` 5.0) false false)
    (`self.Light`)))

(event `Breaking`
  (set `self.CanRotate` false)
  (`AudioComponent.Stop` (`self.emergencyAlarmWithReverb_Cue`))
  (`LightComponent.SetLightColor` :`self` (`self.SpotLight`)))

(fn `UserConstructionScript`)