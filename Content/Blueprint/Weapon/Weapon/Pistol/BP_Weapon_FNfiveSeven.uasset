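; Pistol weapon Blueprint for the FN Five-seveN that implements its procedural reload animation.
; Chained timelines tilt the gun through RecoilTransformDNC, slide the magazine out and away, then play reversed motions to reinsert it and level the gun.
; CurrentHandPos switches between weapon body and magazine during the sequence.
; An empty reload also animates the slide back to its rest position after a short delay.
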(event `self.ReloadingAnimation`
  (params (`Empty?` :type Boolean))
  (set `self.CurrentHandPos` (`self.WeaponBody`))
  (bind (_direction _newtrack_0) (`Timeline|Timeline_5` :!via `PlayFromStart`)
    (:`Update`
      (set `self.RecoilTransformDNC` (`KismetMathLibrary.MakeTransform` (`KismetMathLibrary.VLerp` (0.0 0.0 0.0) (`KismetMathLibrary.MakeVector` 0.0 10.0 10.0) _newtrack_0) (`KismetMathLibrary.RLerp` (struct) (`KismetMathLibrary.MakeRotator` -40.0 10.0 5.0) _newtrack_0))))
    (:`Finished`
      (set `self.CurrentHandPos` (`self.WeaponMag`))
      (bind (_direction_2 _newtrack_0_2) (`Timeline|RemoveMag` :!via `PlayFromStart`)
        (:`Update`
          (`SceneComponent.K2_SetRelativeTransform` (`self.WeaponMag`) (`KismetMathLibrary.TLerp` (`KismetMathLibrary.MakeTransform` (0.0 0.0 0.0)) (`KismetMathLibrary.MakeTransform` (-3.0 0.0 -15.0)) _newtrack_0_2) false false))
        (:`Finished`
          (bind (_direction_3 _newtrack_0_3) (`Timeline|Change` :!via `PlayFromStart`)
            (:`Update`
              (`SceneComponent.K2_SetRelativeTransform` (`self.WeaponMag`) (`KismetMathLibrary.TLerp` (`KismetMathLibrary.MakeTransform` (-3.0 0.0 -15.0)) (`KismetMathLibrary.MakeTransform` (-28.0 -42.0 -35.0) (struct :`Pitch` -8.3 :`Yaw` -18.25 :`Roll` 66.300003)) _newtrack_0_3) false false))
            (:`Finished`
              (bind (_direction_4 _newtrack_0_4) (`Timeline|Timeline_4` :!via `ReverseFromEnd`)
                (:`Update`
                  (`SceneComponent.K2_SetRelativeTransform` (`self.WeaponMag`) (`KismetMathLibrary.TLerp` (`KismetMathLibrary.MakeTransform` (-3.0 0.0 -15.0)) (`KismetMathLibrary.MakeTransform` (-28.0 -42.0 -35.0) (struct :`Pitch` -8.3 :`Yaw` -18.25 :`Roll` 66.300003)) _newtrack_0_4) false false))
                (:`Finished`
                  (bind (_direction_5 _newtrack_0_5) (`Timeline|Timeline_3_0` :!via `ReverseFromEnd`)
                    (:`Update`
                      (`SceneComponent.K2_SetRelativeTransform` (`self.WeaponMag`) (`KismetMathLibrary.TLerp` (`KismetMathLibrary.MakeTransform` (0.0 0.0 0.0)) (`KismetMathLibrary.MakeTransform` (-3.0 0.0 -15.0)) _newtrack_0_5) false false))
                    (:`Finished`
                      (`|ExecutionSequence`
                        (:`then_0`
                          (if `Empty?`
                            (`KismetSystemLibrary.Delay` 0.2)
                            (bind (_direction_6 _recul) (`Timeline|Timeline_6` :!via `ReverseFromEnd`)
                              (:`Update`
                                (`SceneComponent.K2_SetRelativeLocation` (`self.WeaponSlide`) (`KismetMathLibrary.VLerp` (0.0 0.0 0.0) (-5.0 0.0 0.0) _recul) false false)))))
                        (:`then_1`
                          (set `self.CurrentHandPos` (`self.WeaponBody`))
                          (bind (_direction_7 _newtrack_0_6) (`Timeline|Timeline_7` :!via `ReverseFromEnd`)
                            (:`Update`
                              (set `self.RecoilTransformDNC` (`KismetMathLibrary.MakeTransform` (`KismetMathLibrary.VLerp` (0.0 0.0 0.0) (`KismetMathLibrary.MakeVector` 0.0 10.0 10.0) _newtrack_0_6) (`KismetMathLibrary.RLerp` (struct) (`KismetMathLibrary.MakeRotator` -40.0 10.0 5.0) _newtrack_0_6))))))))))))))))))

(fn `UserConstructionScript`
  (`parent.UserConstructionScript`))