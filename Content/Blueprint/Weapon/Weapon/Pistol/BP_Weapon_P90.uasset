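; P90 weapon Blueprint that supplies a procedural reload animation through its ReloadingAnimation event.
; Chained timelines tilt the weapon via RecoilTransformDNC, pull the magazine out and away, then reverse it back in and lower the weapon.
; When the Empty flag is set, a delayed slide pull-and-return also plays, overlapping the lowering.
; CurrentHandPos switches between body, magazine and slide to mark the hand's target at each stage.
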(event `self.ReloadingAnimation`
  (params (`Empty?` :type Boolean))
  (set `self.CurrentHandPos` (`self.WeaponBody`))
  (bind (_direction _newtrack_0) (`Timeline|Timeline_3_0` :!via `PlayFromStart`)
    (:`Update`
      (set `self.RecoilTransformDNC` (`KismetMathLibrary.MakeTransform` (`KismetMathLibrary.VLerp` (0.0 0.0 0.0) (`KismetMathLibrary.MakeVector` 15.0 20.0 40.0) _newtrack_0) (`KismetMathLibrary.RLerp` (struct) (`KismetMathLibrary.MakeRotator` -30.0 -5.0 5.0) _newtrack_0))))
    (:`Finished`
      (set `self.CurrentHandPos` (`self.WeaponMag`))
      (bind (_direction_2 _newtrack_0_2) (`Timeline|Timeline_4` :!via `PlayFromStart`)
        (:`Update`
          (`SceneComponent.K2_SetRelativeTransform` (`self.WeaponMag`) (`KismetMathLibrary.TLerp` (`KismetMathLibrary.MakeTransform` (0.0 0.0 0.0)) (`KismetMathLibrary.MakeTransform` (0.0 47.0 21.0) (struct :`Roll` -20.0)) _newtrack_0_2) false false))
        (:`Finished`
          (bind (_direction_3 _newtrack_0_3) (`Timeline|Timeline_5` :!via `PlayFromStart`)
            (:`Update`
              (`SceneComponent.K2_SetRelativeTransform` (`self.WeaponMag`) (`KismetMathLibrary.TLerp` (`KismetMathLibrary.MakeTransform` (0.0 47.0 21.0) (struct :`Roll` -20.0)) (`KismetMathLibrary.MakeTransform` (-184.0 0.0 -10.0) (struct :`Pitch` 14.0 :`Yaw` 43.25 :`Roll` 15.56)) _newtrack_0_3) false false))
            (:`Finished`
              (bind (_direction_4 _newtrack_0_4) (`Timeline|Timeline_7` :!via `ReverseFromEnd`)
                (:`Update`
                  (`SceneComponent.K2_SetRelativeTransform` (`self.WeaponMag`) (`KismetMathLibrary.TLerp` (`KismetMathLibrary.MakeTransform` (0.0 47.0 21.0) (struct :`Roll` -20.0)) (`KismetMathLibrary.MakeTransform` (-184.0 0.0 -10.0) (struct :`Pitch` 14.0 :`Yaw` 43.25 :`Roll` 15.56)) _newtrack_0_4) false false))
                (:`Finished`
                  (bind (_direction_5 _newtrack_0_5) (`Timeline|Timeline_6` :!via `ReverseFromEnd`)
                    (:`Update`
                      (`SceneComponent.K2_SetRelativeTransform` (`self.WeaponMag`) (`KismetMathLibrary.TLerp` (`KismetMathLibrary.MakeTransform` (0.0 0.0 0.0)) (`KismetMathLibrary.MakeTransform` (0.0 47.0 21.0) (struct :`Roll` -20.0)) _newtrack_0_5) false false))
                    (:`Finished`
                      (`|ExecutionSequence`
                        (:`then_0`
                          (if `Empty?`
                            (`KismetSystemLibrary.Delay` 0.5)
                            (set `self.CurrentHandPos` (`self.WeaponSlide`))
                            (bind (_direction_6 _recul) (`Timeline|Timeline_8` :!via `PlayFromStart`)
                              (:`Update`
                                (`SceneComponent.K2_SetRelativeLocation` (`self.WeaponSlide`) (`KismetMathLibrary.VLerp` (0.0 0.0 0.0) (0.0 14.0 0.0) _recul) false false))
                              (:`Finished`
                                (bind (_direction_7 _recul_2) (`Timeline|Timeline_10` :!via `ReverseFromEnd`)
                                  (:`Update`
                                    (`SceneComponent.K2_SetRelativeLocation` (`self.WeaponSlide`) (`KismetMathLibrary.VLerp` (0.0 0.0 0.0) (0.0 14.0 0.0) _recul_2) false false)))))))
                        (:`then_1`
                          (set `self.CurrentHandPos` (`self.WeaponBody`))
                          (bind (_direction_8 _newtrack_0_6) (`Timeline|Timeline_9` :!via `ReverseFromEnd`)
                            (:`Update`
                              (set `self.RecoilTransformDNC` (`KismetMathLibrary.MakeTransform` (`KismetMathLibrary.VLerp` (0.0 0.0 0.0) (`KismetMathLibrary.MakeVector` 15.0 20.0 40.0) _newtrack_0_6) (`KismetMathLibrary.RLerp` (struct) (`KismetMathLibrary.MakeRotator` -30.0 -5.0 5.0) _newtrack_0_6))))))))))))))))))

(fn `UserConstructionScript`
  (`parent.UserConstructionScript`))