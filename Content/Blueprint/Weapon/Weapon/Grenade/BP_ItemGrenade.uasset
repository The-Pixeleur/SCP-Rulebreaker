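; BP_ItemGrenade is a grenade item that the player can put in or take out of their hands.
; Its Effect event toggles the FirstPersonCharacter's hand state, either clearing the left hand or adding the M67 hand grenade with a reference to this item.
; Parent Tick runs only while the grenade is not Activated.
; The Explode event is an empty stub, and the M67 classes are hard-coded.
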(event `self.Effect`
  (bind _asfirst_person_character (cast `/Game/PlayerBP/Blueprints/FirstPersonCharacter` (`GameplayStatics.GetPlayerPawn` 0)))
  (if (`/Game/PlayerBP/Blueprints/FirstPersonCharacter.GetSomethinInHands?` _asfirst_person_character)
    (set `/Game/PlayerBP/Blueprints/FirstPersonCharacter.GetSomethinInHands?` false _asfirst_person_character)
    (`/Game/PlayerBP/Blueprints/FirstPersonCharacter.RemoveLefthands` _asfirst_person_character)
    (else
      (set `/Game/PlayerBP/Blueprints/FirstPersonCharacter.GetSomethinInHands?` true _asfirst_person_character)
      (`/Game/PlayerBP/Blueprints/FirstPersonCharacter.AddGrenadeTohand` _asfirst_person_character "/Game/Blueprint/Weapon/Weapon/Grenade/FragM67/BP_HandItemGrenadeM67.BP_HandItemGrenadeM67_C" "/Game/Blueprint/Weapon/Weapon/Grenade/FragM67/BP_ItemGrenadeM67.BP_ItemGrenadeM67_C" self))))

(event `self.ReceiveTick`
  (params (DeltaSeconds :type "Float (single-precision)"))
  (if (not (`self.Activated?`))
    (`parent.ReceiveTick` DeltaSeconds)))

(event `Explode`)

(fn `UserConstructionScript`
  (`parent.UserConstructionScript`))