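; Weapon workbench actor where the player modifies their gun's attachments, with input enabled only while inside its trigger box.
; Use spawns a display copy of the held weapon with matching attachments, blends the view to the station and opens UI_WeaponBuild.
; Widget events drive timelines that ease the camera from its current transform to general or per-slot views.
; Removing the gun destroys the copy and returns the camera to the general view.
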(event `self.Box.OnComponentBeginOverlap`
  (params (OverlappedComponent :type "PrimitiveComponent Object Reference") (OtherActor :type "Actor Object Reference") (OtherComp :type "PrimitiveComponent Object Reference") (OtherBodyIndex :type Integer) (bFromSweep :type Boolean) (SweepResult :type "HitResult Structure (by ref)"))
  (bind _asfirst_person_character (cast `/Game/PlayerBP/Blueprints/FirstPersonCharacter` OtherActor))
  (set `self.As First Person Character` _asfirst_person_character)
  (`self.EnableInput` (`GameplayStatics.GetPlayerController` 0)))

(event `self.Box.OnComponentEndOverlap`
  (params (OverlappedComponent :type "PrimitiveComponent Object Reference") (OtherActor :type "Actor Object Reference") (OtherComp :type "PrimitiveComponent Object Reference") (OtherBodyIndex :type Integer))
  (bind _asfirst_person_character (cast `/Game/PlayerBP/Blueprints/FirstPersonCharacter` OtherActor))
  (set `self.As First Person Character` _asfirst_person_character)
  (`self.DisableInput` (`GameplayStatics.GetPlayerController` 0)))

(event `InputAction|Use`
  (params (Key :type "Key Structure"))
  (:`Pressed`
    (`self.StartModification` (`self.As First Person Character`))))

(event `StartModification`
  (params (FPSchar :type "/Game/PlayerBP/Blueprints/FirstPersonCharacter Object Reference"))
  (bind _returnvalue (`GameplayStatics.GetPlayerController` 0))
  (bind _asfirst_person_character (cast `/Game/PlayerBP/Blueprints/FirstPersonCharacter` FPSchar))
  (bind _weaponref (`/Game/PlayerBP/Blueprints/FirstPersonCharacter.WeaponRef` _asfirst_person_character))
  (bind _returnvalue_2 (`|SpawnActorFromClass` (`GameplayStatics.GetObjectClass` _weaponref) (`SceneComponent.K2_GetComponentToWorld` (`self.Box1`)) "Undefined" "OverrideRootScale" null null))
  (bind _output_get (set `self.NewVar_0` _returnvalue_2))
  (`|ExecutionSequence`
    (:`then_0`
      (`PlayerController.SetViewTargetWithBlend` _returnvalue self 0.25 "VTBlend_Linear" 0.25 false)
      (bind _returnvalue_3 (`|CreateWidget` "/Game/UI/Weapon/UI_WeaponBuild.UI_WeaponBuild_C" null _weaponref (`self.NewVar_0`)))
      (`UserWidget.AddToPlayerScreen` _returnvalue_3 0)
      (`WidgetBlueprintLibrary.SetInputMode_UIOnlyEx` _returnvalue null)
      (set `PlayerController.bShowMouseCursor` true _returnvalue)
      (add `/Game/UI/Weapon/UI_WeaponBuild.RemoveGun` _returnvalue_3 (delegate `Removegun`))
      (add `/Game/UI/Weapon/UI_WeaponBuild.GoToGeneral` _returnvalue_3 (delegate `MoveCamToGeneral`))
      (add `/Game/UI/Weapon/UI_WeaponBuild.GoToBottom` _returnvalue_3 (delegate `MoveCamToBottom`))
      (add `/Game/UI/Weapon/UI_WeaponBuild.GoToTip` _returnvalue_3 (delegate `MoveCamToTip`))
      (add `/Game/UI/Weapon/UI_WeaponBuild.GoToSide` _returnvalue_3 (delegate `MoveCamToSide`))
      (add `/Game/UI/Weapon/UI_WeaponBuild.GoToTop` _returnvalue_3 (delegate `MoveCamToTop`)))
    (:`then_1`
      (bind _topattachment (`/Game/Blueprint/Weapon/BP_Weapon_Master.TopAttachment` _weaponref))
      (`/Game/Blueprint/Weapon/BP_Weapon_Master.SetAttachment` _output_get (`/Game/Blueprint/Weapon/BP_Weapon_Master.TopAttachment` _output_get) (`StaticMeshComponent.StaticMesh` _topattachment) (`SceneComponent.GetRelativeTransform` _topattachment))
      (bind _sideattachment (`/Game/Blueprint/Weapon/BP_Weapon_Master.SideAttachment` _weaponref))
      (`/Game/Blueprint/Weapon/BP_Weapon_Master.SetAttachment` _output_get (`/Game/Blueprint/Weapon/BP_Weapon_Master.SideAttachment` _output_get) (`StaticMeshComponent.StaticMesh` _sideattachment) (`SceneComponent.GetRelativeTransform` _sideattachment))
      (bind _tipattachment (`/Game/Blueprint/Weapon/BP_Weapon_Master.TipAttachment` _weaponref))
      (`/Game/Blueprint/Weapon/BP_Weapon_Master.SetAttachment` _output_get (`/Game/Blueprint/Weapon/BP_Weapon_Master.TipAttachment` _output_get) (`StaticMeshComponent.StaticMesh` _tipattachment) (`SceneComponent.GetRelativeTransform` _tipattachment))
      (bind _bottomattachment (`/Game/Blueprint/Weapon/BP_Weapon_Master.BottomAttachment` _weaponref))
      (`/Game/Blueprint/Weapon/BP_Weapon_Master.SetAttachment` _output_get (`/Game/Blueprint/Weapon/BP_Weapon_Master.BottomAttachment` _output_get) (`StaticMeshComponent.StaticMesh` _bottomattachment) (`SceneComponent.GetRelativeTransform` _bottomattachment)))))

(event `Removegun`
  (bind _camera (`self.Camera`))
  (`self.K2_DestroyActor` (`self.NewVar_0`))
  (bind (_direction _newtrack_1) (`Timeline|GoToGeneral` :!via `PlayFromStart` :!label _label)
    (:`Update`
      (`SceneComponent.K2_SetRelativeTransform` _camera (`KismetMathLibrary.TLerp` (`SceneComponent.GetRelativeTransform` _camera) (`KismetMathLibrary.MakeTransform` (-10.0 100.0 100.0) (struct :`Pitch` -9.5 :`Yaw` -74.5 :`Roll` -2.5)) _newtrack_1) false false))))

(event `MoveCamToGeneral`
  (goto _label :!via `PlayFromStart`))

(event `MoveCamToBottom`
  (bind _camera (`self.Camera`))
  (bind (_direction _newtrack_1) (`Timeline|Timeline_0` :!via `PlayFromStart`)
    (:`Update`
      (`SceneComponent.K2_SetRelativeTransform` _camera (`KismetMathLibrary.TLerp` (`SceneComponent.GetRelativeTransform` _camera) (`KismetMathLibrary.MakeTransform` (-35.75 56.5 73.5) (struct :`Pitch` 12.0 :`Yaw` -24.0 :`Roll` 0.4)) _newtrack_1) false false))))

(event `MoveCamToTop`
  (bind _camera (`self.Camera`))
  (bind (_direction _newtrack_1) (`Timeline|Timeline_1` :!via `PlayFromStart`)
    (:`Update`
      (`SceneComponent.K2_SetRelativeTransform` _camera (`KismetMathLibrary.TLerp` (`SceneComponent.GetRelativeTransform` _camera) (`KismetMathLibrary.MakeTransform` (-8.0 63.5 104.0) (struct :`Pitch` -15.0 :`Yaw` -60.0 :`Roll` -7.0)) _newtrack_1) false false))))

(event `MoveCamToTip`
  (bind _camera (`self.Camera`))
  (bind (_direction _newtrack_1) (`Timeline|Timeline_2` :!via `PlayFromStart`)
    (:`Update`
      (`SceneComponent.K2_SetRelativeTransform` _camera (`KismetMathLibrary.TLerp` (`SceneComponent.GetRelativeTransform` _camera) (`KismetMathLibrary.MakeTransform` (-35.0 80.0 99.5) (struct :`Pitch` -18.5 :`Yaw` -49.0 :`Roll` -1.5)) _newtrack_1) false false))))

(event `MoveCamToSide`
  (bind _camera (`self.Camera`))
  (bind (_direction _newtrack_1) (`Timeline|Timeline_3` :!via `PlayFromStart`)
    (:`Update`
      (`SceneComponent.K2_SetRelativeTransform` _camera (`KismetMathLibrary.TLerp` (`SceneComponent.GetRelativeTransform` _camera) (`KismetMathLibrary.MakeTransform` (-20.0 17.5 84.0) (struct :`Pitch` 5.0 :`Yaw` 30.0 :`Roll` 0.4)) _newtrack_1) false false))))

(fn `UserConstructionScript`)